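; FloorSwitcher_BP is a floor switch that drives the vertical movement of a button and a door.
; BeginPlay sets each part's travel distance, and separate events play or reverse a timeline for each.
; Timeline updates lerp Z from the stored start location by that distance and pass it to the location update calls.
; No trigger logic links button to door in this graph.
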(event EventRaiseButton
  (bind _buttonstartlocation (Variables|Default|GetButtonStartLocation))
  (bind _timelinetrack (Timeline|Timeline_Button Reverse)
    (:Update
      (Class|FloorSwitcher|UpdateButtonLocation (Math|Float|Lerp (.z _buttonstartlocation) (+ (.z _buttonstartlocation) (Variables|Default|GetButtonEndPlace)) _timelinetrack)))))

(event EventLoweringButton
  (bind _buttonstartlocation (Variables|Default|GetButtonStartLocation))
  (bind _timelinetrack (Timeline|Timeline_Button Play)
    (:Update
      (Class|FloorSwitcher|UpdateButtonLocation (Math|Float|Lerp (.z _buttonstartlocation) (+ (.z _buttonstartlocation) (Variables|Default|GetButtonEndPlace)) _timelinetrack)))))

(event EventBeginPlay
  (Variables|Default|SetButtonEndPlace 3e+01)
  (Variables|Default|SetDoorEndPlace 3e+02))

(event EventRaiseDoor
  (bind _doorstartlocation (Variables|Default|GetDoorStartLocation))
  (bind _timelinetrack (Timeline|Timeline_Door Play)
    (:Update
      (Class|FloorSwitcher|UpdateDoorLocation (Math|Float|Lerp (.z _doorstartlocation) (+ (.z _doorstartlocation) (Variables|Default|GetDoorEndPlace)) _timelinetrack)))))

(event EventLowerDoor
  (bind _doorstartlocation (Variables|Default|GetDoorStartLocation))
  (bind _timelinetrack (Timeline|Timeline_Door Reverse)
    (:Update
      (Class|FloorSwitcher|UpdateDoorLocation (Math|Float|Lerp (.z _doorstartlocation) (+ (.z _doorstartlocation) (Variables|Default|GetDoorEndPlace)) _timelinetrack)))))

(fn ConstructionScript)