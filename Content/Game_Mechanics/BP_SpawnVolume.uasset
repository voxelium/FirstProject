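; BP_SpawnVolume is a spawn volume that creates an actor along with a temporary particle effect.
; On BeginPlay it spawns ActorToSpawn with random yaw and an emitter, each using its own GetSpawnPoint call, then destroys the emitter after a short delay.
; The SpawnOurPawn override adds the same timed emitter around the parent implementation, noted as C++, but its call in this graph is disconnected.
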(event EventBeginPlay
  ;[1 1 1] Spawn actor in random point of SpawnVolume ver 1
  (bind _returnvalue (Effects|SpawnEmitteratLocation "/Engine/Tutorial/SubEditors/TutorialAssets/TutorialParticleSystem.TutorialParticleSystem" (Class|SpawnVolume|GetSpawnPoint)))
  (Variables|Default|Setref_Particles _returnvalue)
  (Game|SpawnActorfromClass (Variables|Default|GetActorToSpawn) (Math|Transform|MakeTransform (Class|SpawnVolume|GetSpawnPoint) (Math|Rotator|MakeRotator 0.0 0.0 (Math|Random|RandomFloatinRange 0.0 359.0)) "1.000000,1.000000,1.000000") "Undefined" 0 0)
  (Utilities|FlowControl|Delay 3.0)
  (Components|DestroyComponent (Variables|Default|Getref_Particles)))

(event EventSpawnOurPawn
  (params (ToSpawn :type Object%20Class%20Reference) (Location :type Vector%20%28by%20ref%29 :default "0, 0, 0"))
  ;[1 1 1] Spawn actor ver 2 / Spawn Actor in C++
  (bind _returnvalue (Effects|SpawnEmitteratLocation "/Engine/Tutorial/SubEditors/TutorialAssets/TutorialParticleSystem.TutorialParticleSystem" Location))
  (Variables|Default|Setref_Particles _returnvalue)
  (|CallParentFunction ToSpawn Location)
  (Utilities|FlowControl|Delay 3.0)
  (Components|DestroyComponent (Variables|Default|Getref_Particles)))

(fn ConstructionScript)